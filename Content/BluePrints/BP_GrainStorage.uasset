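; BP_GrainStorage is a grain store actor that Tribbles eat from, with a widget bar showing the remaining grain.
; Overlapping Tribbles in mode 0 are registered and told to start eating, then removed and stopped when they leave.
; EatGrain removes one grain, clamped at zero, and refreshes the bar.
; NotifyTribbleDied unregisters the dead Tribble and sends the remaining eaters into panic.
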(event `self.ReceiveBeginPlay`
  (`self.UpdateWidget`))

(event `self.ReceiveActorBeginOverlap`
  (params (OtherActor :type "Actor Object Reference"))
  (bind _asbp_tribble_01 (cast `/Game/BluePrints/BP_Tribble_01` OtherActor))
  (if (== (`/Game/BluePrints/BP_Tribble_01.TribbleMode` _asbp_tribble_01) 0)
    (`self.RegisterEatingTribble` _asbp_tribble_01)))

(event `self.ReceiveActorEndOverlap`
  (params (OtherActor :type "Actor Object Reference"))
  (`KismetArrayLibrary.Array_RemoveItem` (`self.EatingTribbles`) OtherActor)
  (bind _asbp_tribble_01 (cast `/Game/BluePrints/BP_Tribble_01` OtherActor))
  (`/Game/BluePrints/BP_Tribble_01.StopEating` _asbp_tribble_01))

(fn `EatGrain`
  (set `self.GrainCount` (`KismetMathLibrary.Clamp` (- (`self.GrainCount`) 1) 0 (`self.MaxGrains`)))
  (`self.UpdateWidget`))

(fn `NotifyTribbleDied`
  (params (DeadTribble :type "Actor Object Reference"))
  (`KismetArrayLibrary.Array_RemoveItem` (`self.EatingTribbles`) DeadTribble)
  (for _array_element (`self.EatingTribbles`)
    (`/Engine/EditorBlueprintResources/StandardMacros.IsValid` _array_element
      (:`Is Valid`
        (bind _asbp_tribble_01 (cast `/Game/BluePrints/BP_Tribble_01` _array_element))
        (`/Game/BluePrints/BP_Tribble_01.StartPanic` _asbp_tribble_01)))))

(fn `RegisterEatingTribble`
  (params (Tribble :type "Actor Object Reference"))
  (`KismetArrayLibrary.Array_Add` (`self.EatingTribbles`) Tribble)
  (bind _asbp_tribble_01 (cast `/Game/BluePrints/BP_Tribble_01` Tribble))
  (`/Game/BluePrints/BP_Tribble_01.StartEating` _asbp_tribble_01 self))

(fn `UpdateWidget`
  (bind _aswbp_grain_health_bar (cast `/Game/BluePrints/WBP_GrainHealthBar` (`WidgetComponent.GetUserWidgetObject` (`self.GrainWidget1`))))
  (`/Game/BluePrints/WBP_GrainHealthBar.SetGrainDisplay` _aswbp_grain_health_bar (`self.GrainCount`) (`self.MaxGrains`)))

(fn `UserConstructionScript`)