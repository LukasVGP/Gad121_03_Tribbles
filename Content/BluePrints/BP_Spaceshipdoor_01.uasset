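; Spaceship door that the player toggles with E when within range and unlocked, with a prompt that turns to face them.
; Opening chains two timelines, rotating the door on pitch, then sliding it along the actor's forward vector; closing reverses both in opposite order.
; A 45-second timer auto-closes it unless MissionUnlocked is set.
; The OpenDoor event sets that flag and clears Locked, so timed closing no longer applies.
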(event `self.ReceiveBeginPlay`
  (set `self.InitialDoorWorldLocation` (`SceneComponent.K2_GetComponentLocation` (`self.SpacehshipDoor`)))
  (`self.EnableInput` (`GameplayStatics.GetPlayerController` 0)))

(event `self.ReceiveActorBeginOverlap`
  (params (OtherActor :type "Actor Object Reference"))
  (cast `Pawn` OtherActor)
  (set `self.bPlayerInRange` true)
  (`SceneComponent.SetVisibility` (`self.InteractionPrompt`) true false))

(event `self.ReceiveActorEndOverlap`
  (params (OtherActor :type "Actor Object Reference")))

(event `Key|E`
  (params (Key :type "Key Structure")))

(event `CloseDoor`
  (if (`self.bMissionUnlocked`)
    _
    (elif (`self.bIsOpen`)
      (set `self.bIsOpen` false :!label _label)
      (`GameplayStatics.PlaySoundAtLocation` "/Game/Soundeffects/Spaceshipdooropensound.Spaceshipdooropensound" (`self.K2_GetActorLocation`) (struct) 1.0 1.0 0.0 null null null null)
      (bind (_direction _newtrack_0) (`Timeline|Timeline_2` :!via `ReverseFromEnd` :!label _label_2)
        (:`Update`
          (`SceneComponent.K2_SetWorldLocation` (`self.SpacehshipDoor`) (+ (`self.InitialDoorWorldLocation`) (* (`self.GetActorForwardVector`) (* _newtrack_0 400.0))) false false))
        (:`Finished`
          (if (not (`self.bIsOpen`))
            (bind (_direction_2 _newtrack_0_2) (`Timeline|Timeline_1` :!via `ReverseFromEnd` :!label _label_3)
              (:`Update`
                (`SceneComponent.K2_SetRelativeRotation` (`self.SpacehshipDoor`) (`KismetMathLibrary.MakeRotator` 0.0 (* (.x _newtrack_0_2) 360.0)) false false))
              (:`Finished`
                (if (`self.bIsOpen`)
                  (goto _label_2))))))))))

(event `OpenDoor`
  (set `self.bMissionUnlocked` true)
  (set `self.bLocked` false)
  (if (not (`self.bIsOpen`)) :!label _label_4
    (set `self.bIsOpen` true)
    (`KismetSystemLibrary.K2_SetTimerDelegate` (delegate `CloseDoor`) 45.0)
    (`GameplayStatics.PlaySoundAtLocation` "/Game/Soundeffects/Spaceshipdooropensound.Spaceshipdooropensound" (`self.K2_GetActorLocation`) (struct) 1.0 1.0 0.0 null null null null)
    (goto _label_3)))

(event `self.ReceiveTick`
  (params (DeltaSeconds :type "Float (single-precision)"))
  (bind _interactionprompt (`self.InteractionPrompt`))
  (bind _returnvalue (`self.K2_GetActorLocation` (`GameplayStatics.GetPlayerCharacter` 0)))
  (bind _returnvalue_2 (<= (`KismetMathLibrary.VSize` (- (`SceneComponent.K2_GetComponentLocation` (`self.SpacehshipDoor`)) _returnvalue)) 500.0))
  (`SceneComponent.K2_SetWorldRotation` _interactionprompt (`KismetMathLibrary.FindLookAtRotation` (`SceneComponent.K2_GetComponentLocation` _interactionprompt) _returnvalue) false false)
  (set `self.bPlayerInRange` _returnvalue_2)
  (`SceneComponent.SetVisibility` (`self.InteractionPrompt`) _returnvalue_2 false)
  (if (`self.bPlayerInRange`)
    (if (not (`self.bLocked`))
      (if (`PlayerController.WasInputKeyJustPressed` (`GameplayStatics.GetPlayerController` 0) "E")
        (if (`self.bIsOpen`)
          (goto _label)
          (else
            (goto _label_4)))))))

(fn `UserConstructionScript`)