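; Rifle weapon Blueprint that supplies the rifle's firing sound and visible gun mesh.
; The OnWeaponFired event plays the rifle shot sound at the actor's location.
; The construction script attaches GunMesh to FPWeapon with collision disabled, then hides FPWeapon in game without propagating to children, so GunMesh stands in as the visible weapon.
; BeginPlay, overlap and Tick are disabled stubs.
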(event `self.OnWeaponFired`
  (`GameplayStatics.PlaySoundAtLocation` (`self.RifleShootSound`) (`self.K2_GetActorLocation`) (struct) 1.0 1.0 0.0 null null null null))

(fn `UserConstructionScript`
  (bind _gunmesh (`self.GunMesh`))
  (bind _fp_weapon (`self.FP_Weapon`))
  (`parent.UserConstructionScript`)
  (`SceneComponent.K2_AttachToComponent` _gunmesh _fp_weapon "None" "KeepRelative" "KeepRelative" "KeepRelative" true)
  (`PrimitiveComponent.SetCollisionEnabled` _gunmesh "NoCollision")
  (`SceneComponent.SetHiddenInGame` _fp_weapon true false))