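; Trigger actor that spawns a wave of random tribbles around itself and reports to the mission manager when finished.
; StartSpawning resets the count and arms it; the next Pawn overlap disarms it and starts a looping timer.
; Each tick of that timer spawns a random class from TribbleClasses at a random XY offset.
; Once SpawnCount is reached, it clears the timer and calls OnSpawnerFinished on BP_MissionManager.
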(event `self.ReceiveActorBeginOverlap`
  (params (OtherActor :type "Actor Object Reference"))
  (cast `Pawn` OtherActor)
  (if (`self.bReadyToSpawn`)
    (set `self.bReadyToSpawn` false)
    (`KismetSystemLibrary.K2_ClearTimer` self "SpawnNextTribble")
    (bind _returnvalue (`KismetSystemLibrary.K2_SetTimer` self "SpawnNextTribble" (`self.SpawnInterval`) true))
    (set `self.SpawnTimerHandle` _returnvalue)))

(fn `SpawnNextTribble`
  (bind _tribbleclasses (`self.TribbleClasses`))
  (bind _missionmanagerref (`self.MissionManagerRef`))
  (if (>= (`self.SpawnedSoFar`) (`self.SpawnCount`))
    (`KismetSystemLibrary.K2_ClearTimer` self "SpawnNextTribble")
    (`/Engine/EditorBlueprintResources/StandardMacros.IsValid` _missionmanagerref
      (:`Is Valid`
        (bind _asbp_mission_manager (cast `/Game/BluePrints/BP_MissionManager` _missionmanagerref))
        (`/Game/BluePrints/BP_MissionManager.OnSpawnerFinished` _asbp_mission_manager)))
    (else
      (bind _asactor (castclass `Actor` (`|GetArrayItem` _tribbleclasses (`KismetMathLibrary.RandomIntegerInRange` 0 (+ (`KismetArrayLibrary.Array_Length` _tribbleclasses) -1)))))
      (`|SpawnActorFromClass` _asactor (`KismetMathLibrary.MakeTransform` (+ (`self.K2_GetActorLocation`) (`KismetMathLibrary.MakeVector` (`KismetMathLibrary.RandomFloatInRange` -200.0 200.0) (`KismetMathLibrary.RandomFloatInRange` -200.0 200.0)))) "Undefined" "MultiplyWithRoot" null null)
      (bind _result (`/Engine/EditorBlueprintResources/StandardMacros.IncrementInt` (`self.SpawnedSoFar`))
        (:`  `
          (set `self.SpawnedSoFar` _result))))))

(fn `StartSpawning`
  (set `self.SpawnedSoFar` 0)
  (set `self.bReadyToSpawn` true))

(fn `UserConstructionScript`)