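; BP_Tribble_04 is a hopping tribble critter that wanders randomly, flees when the player is near, and can be set on fire.
; Tick selects the mode by distance, moves the actor by world offsets with a sine hop, and pushes overlapping tribbles apart.
; Timers drive wander direction and happy sounds.
; StartFire halts wandering and fleeing, then a delayed burn death spawns ashes and notifies BP_ShooterGameMode, which also counts spawns.
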(event `self.ReceiveBeginPlay`
  (set `self.PlayerRef` (`GameplayStatics.GetPlayerCharacter` self))
  (`self.SetActorTickEnabled` true)
  (set `self.GroundZ` (.z (`self.K2_GetActorLocation`)))
  (bind _asbp_shooter_game_mode (cast `/Game/Variant_Shooter/Blueprints/BP_ShooterGameMode` (`GameplayStatics.GetGameMode`)))
  (`/Game/Variant_Shooter/Blueprints/BP_ShooterGameMode.TribbleSpawned` _asbp_shooter_game_mode)
  (`KismetSystemLibrary.K2_SetTimer` self "PlayHappySound" 3.0 true)
  (`KismetSystemLibrary.K2_SetTimer` self "PickNewWanderDir" 2.5 true))

(event `self.ReceiveActorBeginOverlap`
  (params (OtherActor :type "Actor Object Reference"))
  (if (== OtherActor (`self.PlayerRef`))
    (set `self.IsInProximity` true)))

(event `self.ReceiveActorEndOverlap`
  (params (OtherActor :type "Actor Object Reference"))
  (if (== OtherActor (`self.PlayerRef`))
    (set `self.IsInProximity` false)
    (set `self.DamageTimer` 0.0)))

(event `self.ReceiveTick`
  (params (DeltaSeconds :type "Float (single-precision)"))
  (bind _playerref (`self.PlayerRef`))
  (bind _tribblemode (`self.TribbleMode`))
  (bind _returnvalue (- (`self.K2_GetActorLocation`) (`self.K2_GetActorLocation` _playerref)))
  (if (`KismetSystemLibrary.IsValid` _playerref)
    (if (`self.IsOnFire`)
      _
      (elif (`KismetMathLibrary.InRange_FloatFloat` (`KismetMathLibrary.VSize` _returnvalue) 0.0 350.0)
        (set `self.TribbleMode` 1)
        (else
          (set `self.TribbleMode` 0))))
    (if (`KismetMathLibrary.InRange_IntInt` _tribblemode 0 0)
      (`self.K2_AddActorWorldOffset` (* (* (`self.WanderDir`) (150.0 150.0 150.0)) DeltaSeconds))
      (elif (`KismetMathLibrary.InRange_IntInt` _tribblemode 1 1)
        (`self.K2_AddActorWorldOffset` (* (* (`KismetMathLibrary.Normal` _returnvalue) (`self.MoveSpeed`)) DeltaSeconds))))
    (`self.HandleSeparation` DeltaSeconds)
    (bind _output_get (set `self.HopAccumulator` (+ (`self.HopAccumulator`) DeltaSeconds)))
    (`self.K2_AddActorWorldOffset` (`KismetMathLibrary.MakeVector` 0.0 0.0 (- (+ (`self.GroundZ`) (* (`KismetMathLibrary.Abs` (`KismetMathLibrary.Sin` (* _output_get (`self.HopSpeed`)))) (`self.HopHeight`))) (.z (`self.K2_GetActorLocation`)))))))

(event `self.ReceiveEndPlay`
  (params (EndPlayReason :type "EEndPlayReason Enum" :default "Destroyed")))

(event `StartFire`
  (bind _returnvalue (`self.K2_GetActorLocation`))
  (if (not (`self.IsOnFire`))
    (set `self.IsOnFire` true)
    (set `self.TribbleMode` 2)
    (`GameplayStatics.SpawnEmitterAttached` (`self.FireParticle`) (`self.Tribble_Colider`))
    (`GameplayStatics.PlaySoundAtLocation` (`self.BurnDeathSound`) _returnvalue (struct) 1.0 1.0 0.0 null null null null)
    (`GameplayStatics.PlaySoundAtLocation` (`self.OnFireAmbientSound`) _returnvalue (struct) 1.0 1.0 0.0 null null null null)
    (`KismetSystemLibrary.K2_SetTimer` self "TribbleBurnDeath" 7.0)))

(fn `HandleSeparation`
  (params (DeltaSeconds :type "Float (single-precision)"))
  (bind _tribble_colider (`self.Tribble_Colider`))
  (`/Engine/EditorBlueprintResources/StandardMacros.IsValid` _tribble_colider
    (:`Is Valid`
      (set `self.CachedOverlapping` (`PrimitiveComponent.GetOverlappingActors` _tribble_colider (`GameplayStatics.GetObjectClass` self)))
      (for _array_element (`self.CachedOverlapping`)
        (`/Engine/EditorBlueprintResources/StandardMacros.IsValid` _array_element
          (:`Is Valid`
            (`self.K2_AddActorWorldOffset` (* (`KismetMathLibrary.Normal` (+ (- (`self.K2_GetActorLocation`) (`self.K2_GetActorLocation` _array_element)) (`KismetMathLibrary.MakeVector` (`KismetMathLibrary.RandomFloatInRange` -10.0 10.0) (`KismetMathLibrary.RandomFloatInRange` -10.0 10.0)))) (* (`self.SeparationForce`) DeltaSeconds)))))))))

(fn `OnMultiply`
  (bind _returnvalue (`self.K2_GetActorLocation`))
  (`|SpawnActorFromClass` "/Game/BluePrints/BP_Tribble_01.BP_Tribble_01_C" (`KismetMathLibrary.MakeTransform` (+ _returnvalue (`KismetMathLibrary.MakeVector` (`KismetMathLibrary.RandomFloatInRange` -150.0 150.0) (`KismetMathLibrary.RandomFloatInRange` -150.0 150.0)))) "Undefined" "MultiplyWithRoot" null null)
  (`|SpawnActorFromClass` "/Game/BluePrints/BP_Tribble_01.BP_Tribble_01_C" (`KismetMathLibrary.MakeTransform` (+ _returnvalue (`KismetMathLibrary.MakeVector` (`KismetMathLibrary.RandomFloatInRange` -150.0 150.0) (`KismetMathLibrary.RandomFloatInRange` -150.0 150.0)))) "Undefined" "MultiplyWithRoot" null null))

(fn `PickNewWanderDir`
  (set `self.WanderDir` (`KismetMathLibrary.Normal` (`KismetMathLibrary.MakeVector` (`KismetMathLibrary.RandomFloatInRange` -1.0 1.0) (`KismetMathLibrary.RandomFloatInRange` -1.0 1.0)))))

(fn `PlayHappySound`
  (if (`KismetMathLibrary.InRange_IntInt` (`self.TribbleMode`) 0 0)
    (`GameplayStatics.PlaySoundAtLocation` (`self.HappySound`) (`self.K2_GetActorLocation`) (struct) 1.0 1.0 0.0 null null null null)))

(fn `TribbleBurnDeath`
  (bind _asactor (castclass `Actor` (`self.TribbleAshesClass`)))
  (`|SpawnActorFromClass` _asactor (`KismetMathLibrary.MakeTransform` (`self.K2_GetActorLocation`)) "Undefined" "MultiplyWithRoot" null null)
  (bind _asbp_shooter_game_mode (cast `/Game/Variant_Shooter/Blueprints/BP_ShooterGameMode` (`GameplayStatics.GetGameMode`)))
  (`/Game/Variant_Shooter/Blueprints/BP_ShooterGameMode.TribbleKilled` _asbp_shooter_game_mode)
  (`self.K2_DestroyActor`))

(fn `UserConstructionScript`
  (set `self.WanderDir` (`KismetMathLibrary.MakeVector` 1.0)))