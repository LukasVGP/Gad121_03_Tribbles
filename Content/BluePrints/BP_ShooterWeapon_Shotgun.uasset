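; Shotgun weapon Blueprint that supplies the visual setup and firing effects for a shooter weapon.
; The construction script assigns grenade launcher skeletal meshes to the first- and third-person components but hides them, and disables collision and physics on a separate pipe shotgun mesh.
; On firing, it plays a gunshot sound and attaches two emitters, one of them smoke, to the hidden first-person muzzle socket, deactivating each after a short delay.
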(event `self.OnWeaponFired`
  (bind _fp_weapon (`self.FP_Weapon`))
  (`GameplayStatics.PlaySoundAtLocation` (`self.GunShotSound`) (`self.K2_GetActorLocation`) (struct) 1.0 1.0 0.0 null null null null)
  (bind _returnvalue (`GameplayStatics.SpawnEmitterAttached` null _fp_weapon "Muzzle" (0.0 0.0 0.0) (struct) (0.3 0.3 0.3) "SnapToTarget"))
  (bind _returnvalue_2 (`GameplayStatics.SpawnEmitterAttached` "/Game/StarterContent/Particles/P_Smoke.P_Smoke" _fp_weapon "Muzzle" (0.0 0.0 0.0) (struct) (0.4 0.4 0.4) "SnapToTarget"))
  (`|ExecutionSequence`
    (:`then_0`
      (`KismetSystemLibrary.Delay` 0.5)
      (`/Engine/EditorBlueprintResources/StandardMacros.IsValid` _returnvalue
        (:`Is Valid`
          (`ActorComponent.Deactivate` _returnvalue))))
    (:`then_1`
      (`KismetSystemLibrary.Delay` 1.0)
      (`/Engine/EditorBlueprintResources/StandardMacros.IsValid` _returnvalue_2
        (:`Is Valid`
          (`ActorComponent.Deactivate` _returnvalue_2))))))

(fn `UserConstructionScript`
  (bind _fp_weapon (`self.FP_Weapon`))
  (bind _tp_weapon (`self.TP_Weapon`))
  (bind _pipeshotgunmesh (`self.PipeShotgunMesh`))
  (`parent.UserConstructionScript`)
  (`SkeletalMeshComponent.SetSkeletalMeshAsset` _fp_weapon "/Game/Weapons/GrenadeLauncher/Meshes/SKM_GrenadeLauncher.SKM_GrenadeLauncher")
  (`SkeletalMeshComponent.SetSkeletalMeshAsset` _tp_weapon "/Game/Weapons/GrenadeLauncher/Meshes/SKM_GrenadeLauncher.SKM_GrenadeLauncher")
  (`SceneComponent.SetVisibility` _fp_weapon false false)
  (`SceneComponent.SetVisibility` _tp_weapon false false)
  (`PrimitiveComponent.SetCollisionEnabled` _pipeshotgunmesh "NoCollision")
  (`PrimitiveComponent.SetSimulatePhysics` _pipeshotgunmesh false))