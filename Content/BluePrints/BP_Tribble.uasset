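; BP_Tribble is a hopping enemy that chases the player and deals periodic damage while overlapping them.
; Tick moves it toward the player, pushes it off overlapping tribbles with jittered separation and applies a sine-based hop around its spawn height.
; It reports spawn and end of play to BP_ShooterGameMode as TribbleSpawned and TribbleKilled.
; OnMultiply spawns two more tribbles at random nearby offsets, with no caller in this Blueprint.
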(event `self.ReceiveBeginPlay`
  (set `self.PlayerRef` (`GameplayStatics.GetPlayerCharacter` self))
  (`self.SetActorTickEnabled` true)
  (set `self.GroundZ` (.z (`self.K2_GetActorLocation`)))
  (bind _asbp_shooter_game_mode (cast `/Game/Variant_Shooter/Blueprints/BP_ShooterGameMode` (`GameplayStatics.GetGameMode`)))
  (`/Game/Variant_Shooter/Blueprints/BP_ShooterGameMode.TribbleSpawned` _asbp_shooter_game_mode))

(event `self.ReceiveActorBeginOverlap`
  (params (OtherActor :type "Actor Object Reference"))
  (if (== OtherActor (`self.PlayerRef`))
    (set `self.IsInProximity` true)))

(event `self.ReceiveActorEndOverlap`
  (params (OtherActor :type "Actor Object Reference"))
  (if (== OtherActor (`self.PlayerRef`))
    (set `self.IsInProximity` false)
    (set `self.DamageTimer` 0.0)))

(event `self.ReceiveTick`
  (params (DeltaSeconds :type "Float (single-precision)"))
  (bind _playerref (`self.PlayerRef`))
  (if (`KismetSystemLibrary.IsValid` _playerref)
    (`self.K2_AddActorLocalOffset` self (* (`KismetMathLibrary.GetDirectionUnitVector` (`self.K2_GetActorLocation`) (`self.K2_GetActorLocation` _playerref)) (* (`self.MoveSpeed`) DeltaSeconds)) false false)
    (`self.HandleSeparation` DeltaSeconds)
    (bind _output_get (set `self.HopAccumulator` (+ (`self.HopAccumulator`) DeltaSeconds)))
    (`self.K2_AddActorWorldOffset` (`KismetMathLibrary.MakeVector` 0.0 0.0 (- (+ (`self.GroundZ`) (* (`KismetMathLibrary.Abs` (`KismetMathLibrary.Sin` (* _output_get (`self.HopSpeed`)))) (`self.HopHeight`))) (.z (`self.K2_GetActorLocation`)))))
    (if (`self.IsInProximity`)
      (bind _output_get_2 (set `self.DamageTimer` (+ (`self.DamageTimer`) DeltaSeconds)))
      (if (>= _output_get_2 (`self.DamageInterval`))
        (`GameplayStatics.ApplyDamage` _playerref (`self.ProximityDamage`) null self)
        (set `self.DamageTimer` 0.0)))))

(event `self.ReceiveEndPlay`
  (params (EndPlayReason :type "EEndPlayReason Enum" :default "Destroyed"))
  (bind _asbp_shooter_game_mode (cast `/Game/Variant_Shooter/Blueprints/BP_ShooterGameMode` (`GameplayStatics.GetGameMode`)))
  (`/Game/Variant_Shooter/Blueprints/BP_ShooterGameMode.TribbleKilled` _asbp_shooter_game_mode))

(fn `HandleSeparation`
  (params (DeltaSeconds :type "Float (single-precision)"))
  (for _array_element (`PrimitiveComponent.GetOverlappingActors` (`self.Tribble_Colider`) (`GameplayStatics.GetObjectClass` self))
    (`self.K2_AddActorWorldOffset` (* (`KismetMathLibrary.Normal` (+ (- (`self.K2_GetActorLocation`) (`self.K2_GetActorLocation` _array_element)) (`KismetMathLibrary.MakeVector` (`KismetMathLibrary.RandomFloatInRange` -10.0 10.0) (`KismetMathLibrary.RandomFloatInRange` -10.0 10.0)))) (* (`self.SeparationForce`) DeltaSeconds)))))

(fn `OnMultiply`
  (bind _returnvalue (`self.K2_GetActorLocation`))
  (`|SpawnActorFromClass` "BP_Tribble_C" (`KismetMathLibrary.MakeTransform` (+ _returnvalue (`KismetMathLibrary.MakeVector` (`KismetMathLibrary.RandomFloatInRange` -150.0 150.0) (`KismetMathLibrary.RandomFloatInRange` -150.0 150.0)))) "Undefined" "MultiplyWithRoot" null null)
  (`|SpawnActorFromClass` "BP_Tribble_C" (`KismetMathLibrary.MakeTransform` (+ _returnvalue (`KismetMathLibrary.MakeVector` (`KismetMathLibrary.RandomFloatInRange` -150.0 150.0) (`KismetMathLibrary.RandomFloatInRange` -150.0 150.0)))) "Undefined" "MultiplyWithRoot" null null))

(fn `UserConstructionScript`)