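; BP_ShooterWeapon_TribblePistol is a pistol weapon Blueprint for the shooter, built on a parent weapon class.
; Its construction script gives FPWeapon the pistol skeletal mesh, attaches a collision-free GunMesh to it, and hides FPWeapon in game without propagating to children, so GunMesh shows in its place.
; When the weapon fires, it plays the Tribble pistol shot sound at the actor's location.
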(event `self.OnWeaponFired`
  (`GameplayStatics.PlaySoundAtLocation` (`self.TribblePistolShot`) (`self.K2_GetActorLocation`) (struct) 1.0 1.0 0.0 null null null null))

(fn `UserConstructionScript`
  (bind _fp_weapon (`self.FP_Weapon`))
  (`parent.UserConstructionScript`)
  (`SkeletalMeshComponent.SetSkeletalMeshAsset` _fp_weapon "/Game/Weapons/Pistol/Meshes/SKM_Pistol.SKM_Pistol")
  (`PrimitiveComponent.SetCollisionEnabled` (`self.GunMesh`) "NoCollision")
  (`SceneComponent.K2_AttachToComponent` (`self.GunMesh`) _fp_weapon "None" "KeepRelative" "KeepRelative" "KeepRelative" true)
  (`SceneComponent.SetHiddenInGame` _fp_weapon true false))