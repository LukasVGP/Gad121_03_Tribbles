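; Projectile that multiplies actors tagged "Tribble" on overlap, replacing the hit one with up to two random Tribbles.
; It traces down for ground height, plays a sound, then destroys itself, skipping multiplication once 30 Tribbles exist.
; Two identical helpers spawn at random offsets, re-rolling at each nested compare, so variant odds are uneven and spawns can fail.
; Casts to the four variants set IsMultiplying before the original is destroyed.
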(event `self.ReceiveActorBeginOverlap`
  (params (OtherActor :type "Actor Object Reference"))
  (bind _tribblespawnlocation (`self.TribbleSpawnLocation`))
  (if (`self.ActorHasTag` OtherActor "Tribble")
    (set `self.TribbleSpawnLocation` (`self.K2_GetActorLocation` OtherActor))
    (bind (_outhit _returnvalue) (`KismetSystemLibrary.LineTraceSingle` (`self.TribbleSpawnLocation`) (- (`self.TribbleSpawnLocation`) (`KismetMathLibrary.MakeVector` 0.0 0.0 500.0)) "TraceTypeQuery1"))
    (if _returnvalue
      (set `self.TribbleSpawnLocation` (`KismetMathLibrary.MakeVector` (.x (`self.TribbleSpawnLocation`)) (.y (`self.TribbleSpawnLocation`)) (.z (`.Location` (`GameplayStatics.BreakHitResult` _outhit))))))
    (`GameplayStatics.PlaySoundAtLocation` (`self.DoubleSound`) _tribblespawnlocation (struct) 1.0 1.0 0.0 null null null null)
    (bind _outactors (`GameplayStatics.GetAllActorsWithTag` "Tribble"))
    (if (>= (`KismetArrayLibrary.Array_Length` _outactors) 30)
      (`self.K2_DestroyActor`)
      (else
        (`self.SpawnFirstTribble` (`KismetMathLibrary.MakeTransform` (+ _tribblespawnlocation (`KismetMathLibrary.MakeVector` (`KismetMathLibrary.RandomFloatInRange` -150.0 150.0) (`KismetMathLibrary.RandomFloatInRange` -150.0 150.0)))))
        (`self.SpawnSecondTribble` (`KismetMathLibrary.MakeTransform` (+ _tribblespawnlocation (`KismetMathLibrary.MakeVector` (`KismetMathLibrary.RandomFloatInRange` -150.0 150.0) (`KismetMathLibrary.RandomFloatInRange` -150.0 150.0)))))
        (bind _asbp_tribble_01 (cast `/Game/BluePrints/BP_Tribble_01` OtherActor)
          (:`then`
            (set `/Game/BluePrints/BP_Tribble_01.IsMultiplying` true _asbp_tribble_01)
            (`self.K2_DestroyActor` OtherActor)
            (`self.K2_DestroyActor`))
          (:`CastFailed`
            (bind _asbp_tribble_02 (cast `/Game/BluePrints/BP_Tribble_02` OtherActor)
              (:`then`
                (set `/Game/BluePrints/BP_Tribble_02.IsMultiplying` true _asbp_tribble_02)
                (`self.K2_DestroyActor` OtherActor)
                (`self.K2_DestroyActor`))
              (:`CastFailed`
                (bind _asbp_tribble_03 (cast `/Game/BluePrints/BP_Tribble_03` OtherActor)
                  (:`then`
                    (set `/Game/BluePrints/BP_Tribble_03.IsMultiplying` true _asbp_tribble_03)
                    (`self.K2_DestroyActor` OtherActor)
                    (`self.K2_DestroyActor`))
                  (:`CastFailed`
                    (bind _asbp_tribble_04 (cast `/Game/BluePrints/BP_Tribble_04` OtherActor)
                      (:`then`
                        (set `/Game/BluePrints/BP_Tribble_04.IsMultiplying` true _asbp_tribble_04))
                      (:`CastFailed`
                        _))
                    (`self.K2_DestroyActor` OtherActor)
                    (`self.K2_DestroyActor`)))))))))))

(fn `SpawnFirstTribble`
  (params (SpawnTransform :type "Transform Structure"))
  (bind _returnvalue (`KismetMathLibrary.RandomIntegerInRange` 0 3))
  (`/Engine/EditorBlueprintResources/StandardMacros.CompareInt` _returnvalue
    (:`>`
      (`/Engine/EditorBlueprintResources/StandardMacros.CompareInt` _returnvalue 1
        (:`>`
          (`/Engine/EditorBlueprintResources/StandardMacros.CompareInt` _returnvalue 2
            (:`>`
              (`|SpawnActorFromClass` "/Game/BluePrints/BP_Tribble_04.BP_Tribble_04_C" SpawnTransform "Undefined" "MultiplyWithRoot" null null))
            (:`==`
              (`|SpawnActorFromClass` "/Game/BluePrints/BP_Tribble_03.BP_Tribble_03_C" SpawnTransform "Undefined" "MultiplyWithRoot" null null))))
        (:`==`
          (`|SpawnActorFromClass` "/Game/BluePrints/BP_Tribble_02.BP_Tribble_02_C" SpawnTransform "Undefined" "MultiplyWithRoot" null null))))
    (:`==`
      (`|SpawnActorFromClass` "/Game/BluePrints/BP_Tribble_01.BP_Tribble_01_C" SpawnTransform "Undefined" "MultiplyWithRoot" null null))))

(fn `SpawnSecondTribble`
  (params (SpawnTransform :type "Transform Structure"))
  (bind _returnvalue (`KismetMathLibrary.RandomIntegerInRange` 0 3))
  (`/Engine/EditorBlueprintResources/StandardMacros.CompareInt` _returnvalue
    (:`>`
      (`/Engine/EditorBlueprintResources/StandardMacros.CompareInt` _returnvalue 1
        (:`>`
          (`/Engine/EditorBlueprintResources/StandardMacros.CompareInt` _returnvalue 2
            (:`>`
              (`|SpawnActorFromClass` "/Game/BluePrints/BP_Tribble_04.BP_Tribble_04_C" SpawnTransform "Undefined" "MultiplyWithRoot" null null))
            (:`==`
              (`|SpawnActorFromClass` "/Game/BluePrints/BP_Tribble_03.BP_Tribble_03_C" SpawnTransform "Undefined" "MultiplyWithRoot" null null))))
        (:`==`
          (`|SpawnActorFromClass` "/Game/BluePrints/BP_Tribble_02.BP_Tribble_02_C" SpawnTransform "Undefined" "MultiplyWithRoot" null null))))
    (:`==`
      (`|SpawnActorFromClass` "/Game/BluePrints/BP_Tribble_01.BP_Tribble_01_C" SpawnTransform "Undefined" "MultiplyWithRoot" null null))))

(fn `UserConstructionScript`
  (`parent.UserConstructionScript`))