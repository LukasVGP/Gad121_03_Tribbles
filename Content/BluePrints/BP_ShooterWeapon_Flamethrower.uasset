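; Flamethrower shooter weapon that fires a timed burst of attached flame particles and looping-style audio, followed by a cooldown.
; OnWeaponFired starts the effects, and releasing the trigger or hitting the burst timer stops them and starts the cooldown.
; Tick detects the release and aims the flame along player 0's control rotation.
; Cooldown end backdates TimeOfLastShot to bypass the refire delay; no damage logic appears here.
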(event `self.OnWeaponFired`
  (if (and (not (`self.CooldownActive`)) (not (`self.IsCurrentlyFiring`)))
    (set `self.IsCurrentlyFiring` true)
    (bind _returnvalue (`GameplayStatics.SpawnEmitterAttached` (`self.FlameParticleTemplate`) (`self.FP_Weapon`) "Muzzle"))
    (set `self.ActiveFlameEffect` _returnvalue)
    (bind _returnvalue_2 (`GameplayStatics.SpawnSoundAttached` (`self.FlameBurstSound`) (`self.FP_Weapon`) "None" (0.0 0.0 0.0) (struct) "KeepRelativeOffset" false 1.0 1.0 0.0 null null))
    (set `self.FlameAudioComp` _returnvalue_2)
    (bind _returnvalue_3 (`KismetSystemLibrary.K2_SetTimerDelegate` (delegate `ForcedBurstStop`) 5.0))
    (set `self.BurstTimerHandle` _returnvalue_3)))

(event `ForcedBurstStop`
  (`self.DoStopFlame`))

(event `DoStopFlame`
  (`/Engine/EditorBlueprintResources/StandardMacros.IsValid` (`self.ActiveFlameEffect`)
    (:`Is Valid`
      (`ActorComponent.Deactivate` (`self.ActiveFlameEffect`))
      (set `self.ActiveFlameEffect` null))
    (:`Is Not Valid`
      _))
  (`/Engine/EditorBlueprintResources/StandardMacros.IsValid` (`self.FlameAudioComp`)
    (:`Is Valid`
      (`AudioComponent.Stop` (`self.FlameAudioComp`))
      (set `self.FlameAudioComp` null))
    (:`Is Not Valid`
      _))
  (`KismetSystemLibrary.K2_ClearAndInvalidateTimerHandle` (`self.BurstTimerHandle`))
  (set `self.IsCurrentlyFiring` false)
  (set `self.CooldownActive` true)
  (bind _returnvalue (`KismetSystemLibrary.K2_SetTimerDelegate` (delegate `EndCooldown`) 3.0))
  (set `self.CooldownTimerHandle` _returnvalue)
  (`self.Stop Firing`))

(event `EndCooldown`
  (set `self.CooldownActive` false)
  (set `self.Time of Last Shot` (- (`KismetSystemLibrary.GetGameTimeInSeconds`) (+ (`self.Refire Rate`) 1.0))))

(event `self.ReceiveTick`
  (params (DeltaSeconds :type "Float (single-precision)"))
  (bind _iscurrentlyfiring (`self.IsCurrentlyFiring`))
  (bind _is_firing (`self.Is Firing`))
  (`|ExecutionSequence`
    (:`then_0`
      (if (and _iscurrentlyfiring (not _is_firing))
        (`self.DoStopFlame`)))
    (:`then_1`
      (if (and _iscurrentlyfiring _is_firing)
        (`/Engine/EditorBlueprintResources/StandardMacros.IsValid` (`self.ActiveFlameEffect`)
          (:`Is Valid`
            (`SceneComponent.K2_SetWorldRotation` (`self.ActiveFlameEffect`) (`Controller.GetControlRotation` (`GameplayStatics.GetPlayerController` 0)) false false)))))))

(event `self.ReceiveBeginPlay`
  (bind _returnvalue (`self.GetOwner`))
  (message `/Game/Variant_Shooter/Blueprints/Pickups/BPI_WeaponHolder.Attach Weapon Meshes` _returnvalue self (`self.FP_Weapon`) (`self.TP_Weapon`))
  (bind _aspawn (cast `Pawn` _returnvalue)
    (:`then`
      (set `self.Pawn Owner` _aspawn))
    (:`CastFailed`
      _))
  (`|ExecutionSequence`
    (:`then_0`
      (set `self.CooldownActive` false))
    (:`then_1`
      (set `self.IsCurrentlyFiring` false)
      (set `self.Time of Last Shot` (- (`KismetSystemLibrary.GetGameTimeInSeconds`) (+ (`self.Refire Rate`) 1.0))))))

(fn `UserConstructionScript`
  (`parent.UserConstructionScript`))