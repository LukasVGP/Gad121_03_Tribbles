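; Flame projectile actor that kills actors tagged "Tribble" on impact.
; On such a hit it spawns BP_TribbleFlesh and plays a death sound at the victim's location, reports the kill to BP_ShooterGameMode, then destroys both actors.
; Any other hit only destroys the projectile; a failed game mode cast leaves both projectile and Tribble alive.
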(event `self.On Projectile Hit`
  (params (Hit :type "HitResult Structure (by ref)"))
  (bind (_bblockinghit _binitialoverlap _time _distance _location _impactpoint _normal _impactnormal _physmat _hitactor) (`GameplayStatics.BreakHitResult` Hit))
  (bind _returnvalue (`self.K2_GetActorLocation` _hitactor))
  (if (`self.ActorHasTag` _hitactor "Tribble")
    (`|SpawnActorFromClass` "/Game/BluePrints/BP_TribbleFlesh.BP_TribbleFlesh_C" (`KismetMathLibrary.MakeTransform` _returnvalue) "Undefined" "MultiplyWithRoot" null null)
    (`GameplayStatics.PlaySoundAtLocation` (`self.TribbleDeathSound`) _returnvalue (struct) 1.0 1.0 0.0 null null null null)
    (bind _asbp_shooter_game_mode (cast `/Game/Variant_Shooter/Blueprints/BP_ShooterGameMode` (`GameplayStatics.GetGameMode`)))
    (`/Game/Variant_Shooter/Blueprints/BP_ShooterGameMode.TribbleKilled` _asbp_shooter_game_mode)
    (`self.K2_DestroyActor` _hitactor)
    (`self.K2_DestroyActor`)
    (else
      (`self.K2_DestroyActor`))))

(fn `UserConstructionScript`
  (`parent.UserConstructionScript`))