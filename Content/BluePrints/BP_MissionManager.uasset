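; Mission manager that runs five sequential Tribble missions, pushing title, objective and status to BP_ShooterGameMode for the HUD.
; StartMission starts spawners for missions 3–5, whose counting waits for OnSpawnerFinished, and enables grain game-over from mission 2.
; A looping timer polls TribbleCount, fires one-shot count-triggered messages and ends mission 1 at a population target, later ones on extermination.
; EndMission opens that mission's door, then chains the next or triggers the win.
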(event `OnSpawnerFinished`
  (set `self.bCounting` true)
  (set `self.bHadTribbles` false)
  (`self.PushToHUD` (`/Game/Variant_Shooter/Blueprints/BP_ShooterGameMode.MissionTitle` (`self.GameModeRef`)) "All Tribbles are spawned — eliminate them all!" "Tribbles: 0"))

(event `self.ReceiveBeginPlay`
  (bind _asbp_shooter_game_mode (cast `/Game/Variant_Shooter/Blueprints/BP_ShooterGameMode` (`GameplayStatics.GetGameMode`)))
  (set `self.GameModeRef` _asbp_shooter_game_mode)
  (`self.StartMission` 1))

(event `StartNextMission`
  (`self.StartMission` (+ (`self.CurrentMission`) 1)))

(fn `CheckMissionCondition`
  (locals (TribbleCount :type Integer))
  (bind _gamemoderef (`self.GameModeRef`))
  (bind _tribblecount (`local.TribbleCount`))
  (set `local.TribbleCount` (`/Game/Variant_Shooter/Blueprints/BP_ShooterGameMode.TribbleCount` _gamemoderef))
  (`self.CheckTriggerMessages` _tribblecount)
  (`self.PushToHUD` (`/Game/Variant_Shooter/Blueprints/BP_ShooterGameMode.MissionTitle` _gamemoderef) (`/Game/Variant_Shooter/Blueprints/BP_ShooterGameMode.MissionObjective` _gamemoderef) (`KismetTextLibrary.Conv_StringToText` (`KismetStringLibrary.Concat_StrStr` "Tribbles: " (`KismetStringLibrary.Conv_IntToString` _tribblecount))))
  (if (> _tribblecount 0)
    (set `self.bHadTribbles` true))
  (if (`self.bCounting`)
    (`/Engine/EditorBlueprintResources/StandardMacros.CompareInt` (`self.CurrentMission`) 1
      (:`>`
        (if (and (`self.bHadTribbles`) (<= _tribblecount 0))
          (`self.EndMission`)))
      (:`==`
        (if (>= _tribblecount 20)
          (`self.EndMission`)))
      (:`<`
        _)))
  (set `self.LastTribbleCount` _tribblecount))

(fn `CheckTriggerMessages`
  (params (CurrentCount :type Integer))
  (locals (ActiveCounts :type "Array of Integer") (ActiveTexts :type "Array of Text"))
  (bind _currentmission (`self.CurrentMission`))
  (bind _activecounts (`local.ActiveCounts`))
  (bind _firedtriggerindices (`self.FiredTriggerIndices`))
  (`/Engine/EditorBlueprintResources/StandardMacros.CompareInt` _currentmission 1
    (:`>`
      (`/Engine/EditorBlueprintResources/StandardMacros.CompareInt` _currentmission 2
        (:`>`
          (`/Engine/EditorBlueprintResources/StandardMacros.CompareInt` _currentmission 3
            (:`>`
              (`/Engine/EditorBlueprintResources/StandardMacros.CompareInt` _currentmission 4
                (:`>`
                  (set `local.ActiveCounts` (`self.M5_TriggerCounts`))
                  (set `local.ActiveTexts` (`self.M5_TriggerTexts`)))
                (:`==`
                  (set `local.ActiveCounts` (`self.M4_TriggerCounts`))
                  (set `local.ActiveTexts` (`self.M4_TriggerTexts`)))))
            (:`==`
              (set `local.ActiveCounts` (`self.M3_TriggerCounts`))
              (set `local.ActiveTexts` (`self.M3_TriggerTexts`)))))
        (:`==`
          (set `local.ActiveCounts` (`self.M2_TriggerCounts`))
          (set `local.ActiveTexts` (`self.M2_TriggerTexts`)))))
    (:`==`
      (set `local.ActiveCounts` (`self.M1_TriggerCounts`))
      (set `local.ActiveTexts` (`self.M1_TriggerTexts`))))
  (for (_ _array_index) _activecounts
    (if (not (`KismetArrayLibrary.Array_Contains` _firedtriggerindices _array_index))
      (if (== CurrentCount (`|GetArrayItem` _activecounts _array_index))
        (`KismetArrayLibrary.Array_Add` _firedtriggerindices _array_index)
        (`self.PushToHUD` (`/Game/Variant_Shooter/Blueprints/BP_ShooterGameMode.MissionTitle` (`self.GameModeRef`)) (`|GetArrayItem` (`local.ActiveTexts`) _array_index) "! Trigger !")))))

(fn `EndMission`
  (bind _currentmission (`self.CurrentMission`))
  (bind _missiontitle (`/Game/Variant_Shooter/Blueprints/BP_ShooterGameMode.MissionTitle` (`self.GameModeRef`)))
  (`KismetSystemLibrary.K2_ClearTimer` self "CheckMissionCondition")
  (`self.OpenMissionDoor` _currentmission)
  (`/Engine/EditorBlueprintResources/StandardMacros.CompareInt` _currentmission 1
    (:`>`
      (`/Engine/EditorBlueprintResources/StandardMacros.CompareInt` _currentmission 2
        (:`>`
          (`/Engine/EditorBlueprintResources/StandardMacros.CompareInt` _currentmission 3
            (:`>`
              (`/Engine/EditorBlueprintResources/StandardMacros.CompareInt` _currentmission 4
                (:`>`
                  (`self.PushToHUD` _missiontitle (`self.M5_EndText`) "Mission Complete!")
                  (bind _asbp_shooter_game_mode (cast `/Game/Variant_Shooter/Blueprints/BP_ShooterGameMode` (`GameplayStatics.GetGameMode`)))
                  (`/Game/Variant_Shooter/Blueprints/BP_ShooterGameMode.TriggerWin` _asbp_shooter_game_mode))
                (:`==`
                  (`self.PushToHUD` _missiontitle (`self.M4_EndText`) "Mission Complete!")
                  (`KismetSystemLibrary.K2_SetTimer` self "StartNextMission" 4.0 :!label _label))))
            (:`==`
              (`self.PushToHUD` _missiontitle (`self.M3_EndText`) "Mission Complete!")
              (goto _label))))
        (:`==`
          (`self.PushToHUD` _missiontitle (`self.M2_EndText`) "Mission Complete!")
          (goto _label))))
    (:`==`
      (`self.PushToHUD` _missiontitle (`self.M1_EndText`) "Mission Complete!")
      (goto _label))))

(fn `OpenMissionDoor`
  (params (MissionIndex :type Integer))
  (bind _m1_door (`self.M1_Door`))
  (bind _m2_door (`self.M2_Door`))
  (bind _m3_door (`self.M3_Door`))
  (bind _m4_door (`self.M4_Door`))
  (bind _m5_door (`self.M5_Door`))
  (switch `int` MissionIndex
    (:`1`
      (`/Engine/EditorBlueprintResources/StandardMacros.IsValid` _m1_door
        (:`Is Valid`
          (bind _asbp_spaceshipdoor_01 (cast `/Game/BluePrints/BP_Spaceshipdoor_01` _m1_door))
          (`/Game/BluePrints/BP_Spaceshipdoor_01.OpenDoor` _asbp_spaceshipdoor_01))))
    (:`2`
      (`/Engine/EditorBlueprintResources/StandardMacros.IsValid` _m2_door
        (:`Is Valid`
          (bind _asbp_spaceshipdoor_01_2 (cast `/Game/BluePrints/BP_Spaceshipdoor_01` _m2_door))
          (`/Game/BluePrints/BP_Spaceshipdoor_01.OpenDoor` _asbp_spaceshipdoor_01_2))))
    (:`3`
      (`/Engine/EditorBlueprintResources/StandardMacros.IsValid` _m3_door
        (:`Is Valid`
          (bind _asbp_spaceshipdoor_01_3 (cast `/Game/BluePrints/BP_Spaceshipdoor_01` _m3_door))
          (`/Game/BluePrints/BP_Spaceshipdoor_01.OpenDoor` _asbp_spaceshipdoor_01_3))))
    (:`4`
      (`/Engine/EditorBlueprintResources/StandardMacros.IsValid` _m4_door
        (:`Is Valid`
          (bind _asbp_spaceshipdoor_01_4 (cast `/Game/BluePrints/BP_Spaceshipdoor_01` _m4_door))
          (`/Game/BluePrints/BP_Spaceshipdoor_01.OpenDoor` _asbp_spaceshipdoor_01_4))))
    (:`5`
      (`/Engine/EditorBlueprintResources/StandardMacros.IsValid` _m5_door
        (:`Is Valid`
          (bind _asbp_spaceshipdoor_01_5 (cast `/Game/BluePrints/BP_Spaceshipdoor_01` _m5_door))
          (`/Game/BluePrints/BP_Spaceshipdoor_01.OpenDoor` _asbp_spaceshipdoor_01_5))))))

(fn `PushToHUD`
  (params (NewTitle :type Text) (NewObjective :type Text) (NewStatus :type Text))
  (bind _gamemoderef (`self.GameModeRef`))
  (`/Engine/EditorBlueprintResources/StandardMacros.IsValid` _gamemoderef
    (:`Is Valid`
      (set `/Game/Variant_Shooter/Blueprints/BP_ShooterGameMode.MissionTitle` NewTitle _gamemoderef)
      (set `/Game/Variant_Shooter/Blueprints/BP_ShooterGameMode.MissionObjective` NewObjective _gamemoderef)
      (set `/Game/Variant_Shooter/Blueprints/BP_ShooterGameMode.MissionStatus` NewStatus _gamemoderef))))

(fn `StartMission`
  (params (MissionIndex :type Integer))
  (bind _m3_spawner (`self.M3_Spawner`))
  (bind _m4_spawner (`self.M4_Spawner`))
  (bind _m5_spawner (`self.M5_Spawner`))
  (set `self.CurrentMission` MissionIndex)
  (set `self.bCounting` false)
  (set `self.bHadTribbles` false)
  (set `self.LastTribbleCount` -1)
  (`KismetArrayLibrary.Array_Clear` (`self.FiredTriggerIndices`))
  (`/Engine/EditorBlueprintResources/StandardMacros.CompareInt` MissionIndex 2
    (:`>`
      (set `/Game/Variant_Shooter/Blueprints/BP_ShooterGameMode.bGrainGameOverEnabled` true (`self.GameModeRef`) :!label _label))
    (:`==`
      (goto _label))
    (:`<`
      _))
  (`/Engine/EditorBlueprintResources/StandardMacros.CompareInt` MissionIndex 1
    (:`>`
      (`/Engine/EditorBlueprintResources/StandardMacros.CompareInt` MissionIndex 2
        (:`>`
          (`/Engine/EditorBlueprintResources/StandardMacros.CompareInt` MissionIndex 3
            (:`>`
              (`/Engine/EditorBlueprintResources/StandardMacros.CompareInt` MissionIndex 4
                (:`>`
                  (`/Engine/EditorBlueprintResources/StandardMacros.IsValid` _m5_spawner
                    (:`Is Valid`
                      (bind _asbp_tribble_spawner (cast `/Game/BluePrints/BP_TribbleSpawner` _m5_spawner))
                      (`/Game/BluePrints/BP_TribbleSpawner.StartSpawning` _asbp_tribble_spawner))
                    (:`Is Not Valid`
                      _)))
                (:`==`
                  (`/Engine/EditorBlueprintResources/StandardMacros.IsValid` _m4_spawner
                    (:`Is Valid`
                      (bind _asbp_tribble_spawner_2 (cast `/Game/BluePrints/BP_TribbleSpawner` _m4_spawner))
                      (`/Game/BluePrints/BP_TribbleSpawner.StartSpawning` _asbp_tribble_spawner_2))
                    (:`Is Not Valid`
                      _)))))
            (:`==`
              (`/Engine/EditorBlueprintResources/StandardMacros.IsValid` _m3_spawner
                (:`Is Valid`
                  (bind _asbp_tribble_spawner_3 (cast `/Game/BluePrints/BP_TribbleSpawner` _m3_spawner))
                  (`/Game/BluePrints/BP_TribbleSpawner.StartSpawning` _asbp_tribble_spawner_3))
                (:`Is Not Valid`
                  _)))))
        (:`==`
          (set `self.bCounting` true))))
    (:`==`
      (set `self.bCounting` true)))
  (`KismetSystemLibrary.K2_SetTimer` self "CheckMissionCondition" 0.5 true)
  (`/Engine/EditorBlueprintResources/StandardMacros.CompareInt` MissionIndex 1
    (:`>`
      (`/Engine/EditorBlueprintResources/StandardMacros.CompareInt` MissionIndex 2
        (:`>`
          (`/Engine/EditorBlueprintResources/StandardMacros.CompareInt` MissionIndex 3
            (:`>`
              (`/Engine/EditorBlueprintResources/StandardMacros.CompareInt` MissionIndex 4
                (:`>`
                  (`self.PushToHUD` (`self.M5_Title`) (`self.M5_BeginText`) "Mission Active"))
                (:`==`
                  (`self.PushToHUD` (`self.M4_Title`) (`self.M4_BeginText`) "Mission Active"))))
            (:`==`
              (`self.PushToHUD` (`self.M3_Title`) (`self.M3_BeginText`) "Mission Active"))))
        (:`==`
          (`self.PushToHUD` (`self.M2_Title`) (`self.M2_BeginText`) "Mission Active"))))
    (:`==`
      (`self.PushToHUD` (`self.M1_Title`) (`self.M1_BeginText`) "Mission Active"))))

(fn `UserConstructionScript`)