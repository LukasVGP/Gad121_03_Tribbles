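; BP_MissionZone is a kill-count mission stage that tracks Tribble kills toward a required total.
; ActivateZone resets the count and writes the mission title, objective and remaining count to BP_ShooterGameMode.
; OnTribbleKilled updates that status and calls MissionComplete when the target is reached.
; Completion either triggers the win on the last mission or opens the linked spaceship door and advances the game mode to the next mission.
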(fn `ActivateZone`
  (set `self.KillsThisMission` 0)
  (bind _asbp_shooter_game_mode (cast `/Game/Variant_Shooter/Blueprints/BP_ShooterGameMode` (`GameplayStatics.GetGameMode`)))
  (set `/Game/Variant_Shooter/Blueprints/BP_ShooterGameMode.MissionTitle` (`self.MissionTitle`) _asbp_shooter_game_mode)
  (set `/Game/Variant_Shooter/Blueprints/BP_ShooterGameMode.MissionObjective` (`self.MissionObjective`) _asbp_shooter_game_mode)
  (set `/Game/Variant_Shooter/Blueprints/BP_ShooterGameMode.MissionStatus` (`|FormatText` "Tribbles Remaining: {Count}" (`self.RequiredKills`)) _asbp_shooter_game_mode))

(fn `MissionComplete`
  (if (`self.IsLastMission`)
    (bind _asbp_shooter_game_mode (cast `/Game/Variant_Shooter/Blueprints/BP_ShooterGameMode` (`GameplayStatics.GetGameMode`)))
    (`/Game/Variant_Shooter/Blueprints/BP_ShooterGameMode.TriggerWin` _asbp_shooter_game_mode)
    (else
      (bind _asbp_spaceshipdoor_01 (cast `/Game/BluePrints/BP_Spaceshipdoor_01` (`self.DoorActor`)))
      (`/Game/BluePrints/BP_Spaceshipdoor_01.OpenDoor` _asbp_spaceshipdoor_01)
      (bind _asbp_shooter_game_mode_2 (cast `/Game/Variant_Shooter/Blueprints/BP_ShooterGameMode` (`GameplayStatics.GetGameMode`)))
      (`/Game/Variant_Shooter/Blueprints/BP_ShooterGameMode.AdvanceMission` _asbp_shooter_game_mode_2))))

(fn `OnTribbleKilled`
  (bind _output_get (set `self.KillsThisMission` (+ (`self.KillsThisMission`) 1)))
  (bind _asbp_shooter_game_mode (cast `/Game/Variant_Shooter/Blueprints/BP_ShooterGameMode` (`GameplayStatics.GetGameMode`)))
  (set `/Game/Variant_Shooter/Blueprints/BP_ShooterGameMode.MissionStatus` (`|FormatText` "Tribbles Remaining: {Count}" (- (`self.RequiredKills`) _output_get)) _asbp_shooter_game_mode)
  (if (>= (`self.KillsThisMission`) (`self.RequiredKills`))
    (`self.MissionComplete`)))

(fn `UserConstructionScript`)