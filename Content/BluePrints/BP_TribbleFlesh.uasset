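; BP_TribbleFlesh is a physics-driven flesh chunk, apparently debris from a Tribble.
; On BeginPlay it spawns a small emitter and a decal at its location, plays a sound, and enables blocking collision and physics simulation on its mesh.
; After a short delay it plays the TribbleFlesh sound.
; The IgniteFlesh event lets a caller attach a supplied fire effect to the mesh.
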(event `IgniteFlesh`
  (params (FireFX :type "ParticleSystem Object Reference"))
  (`GameplayStatics.SpawnEmitterAttached` FireFX (`self.StaticMesh`)))

(event `self.ReceiveBeginPlay`
  (bind _returnvalue (`self.K2_GetActorLocation`))
  (bind _staticmesh (`self.StaticMesh`))
  (`|ExecutionSequence`
    (:`then_0`
      (`GameplayStatics.SpawnEmitterAtLocation` null _returnvalue (struct) (0.2 0.2 0.2))
      (`GameplayStatics.SpawnDecalAtLocation` null (60.0 60.0 60.0) _returnvalue))
    (:`then_1`
      (`GameplayStatics.PlaySoundAtLocation` null (`self.K2_GetActorLocation`) (struct) 1.0 1.0 0.0 null null null null)
      (`PrimitiveComponent.SetCollisionProfileName` _staticmesh "BlockAll" true)
      (`PrimitiveComponent.SetSimulatePhysics` _staticmesh true)
      (`KismetSystemLibrary.Delay` 0.8)
      (`GameplayStatics.PlaySoundAtLocation` "/Game/Soundeffects/TribbleFlesh.TribbleFlesh" (`self.K2_GetActorLocation`) (struct) 1.0 1.0 0.0 null null null null))))

(fn `UserConstructionScript`)