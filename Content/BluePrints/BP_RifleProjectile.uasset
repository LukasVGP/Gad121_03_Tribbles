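; Rifle projectile that splits a Tribble in two on hit, replacing it with two new random Tribbles.
; On overlap with an actor tagged Tribble, a one-shot flag guards the hit, then a sound plays at the target's location.
; Two helper functions each spawn one of four random Tribble variants, offset to either side along world X.
; The hit Tribble and the projectile are then destroyed.
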(event `self.ReceiveActorBeginOverlap`
  (params (OtherActor :type "Actor Object Reference"))
  (bind _returnvalue (`self.K2_GetActorLocation` OtherActor))
  (if (`self.ActorHasTag` OtherActor "Tribble")
    (if (not (`self.HasProcessedHit`))
      (set `self.HasProcessedHit` true)
      (`GameplayStatics.PlaySoundAtLocation` (`self.DoubleSound`) _returnvalue (struct) 1.0 1.0 0.0 null null null null)
      (`self.SpawnFirstRandom` (`KismetMathLibrary.MakeTransform` (+ _returnvalue (300.0 0.0 0.0))))
      (`self.SpawnSecondRandom` (`KismetMathLibrary.MakeTransform` (+ _returnvalue (-300.0 0.0 0.0))))
      (`/Engine/EditorBlueprintResources/StandardMacros.IsValid` OtherActor
        (:`Is Valid`
          (`self.K2_DestroyActor` OtherActor)
          (`/Engine/EditorBlueprintResources/StandardMacros.IsValid` self
            (:`Is Valid`
              _)))
        (:`Is Not Valid`
          _))
      (`self.K2_DestroyActor` self))))

(fn `SpawnFirstRandom`
  (params (SpawnTransform :type "Transform Structure"))
  (switch `int` (`KismetMathLibrary.RandomIntegerInRange` 0 3)
    (:`Default`
      (`|SpawnActorFromClass` "/Game/BluePrints/BP_Tribble_04.BP_Tribble_04_C" SpawnTransform "Undefined" "MultiplyWithRoot" null null))
    (:`0`
      (`|SpawnActorFromClass` "/Game/BluePrints/BP_Tribble_01.BP_Tribble_01_C" SpawnTransform "Undefined" "MultiplyWithRoot" null null))
    (:`1`
      (`|SpawnActorFromClass` "/Game/BluePrints/BP_Tribble_02.BP_Tribble_02_C" SpawnTransform "Undefined" "MultiplyWithRoot" null null))
    (:`2`
      (`|SpawnActorFromClass` "/Game/BluePrints/BP_Tribble_03.BP_Tribble_03_C" SpawnTransform "Undefined" "MultiplyWithRoot" null null))))

(fn `SpawnSecondRandom`
  (params (SpawnTransform :type "Transform Structure"))
  (switch `int` (`KismetMathLibrary.RandomIntegerInRange` 0 3)
    (:`Default`
      (`|SpawnActorFromClass` "/Game/BluePrints/BP_Tribble_04.BP_Tribble_04_C" SpawnTransform "Undefined" "MultiplyWithRoot" null null))
    (:`0`
      (`|SpawnActorFromClass` "/Game/BluePrints/BP_Tribble_02.BP_Tribble_02_C" SpawnTransform "Undefined" "MultiplyWithRoot" null null))
    (:`1`
      (`|SpawnActorFromClass` "/Game/BluePrints/BP_Tribble_03.BP_Tribble_03_C" SpawnTransform "Undefined" "MultiplyWithRoot" null null))
    (:`2`
      (`|SpawnActorFromClass` "/Game/BluePrints/BP_Tribble_01.BP_Tribble_01_C" SpawnTransform "Undefined" "MultiplyWithRoot" null null))))

(fn `UserConstructionScript`)