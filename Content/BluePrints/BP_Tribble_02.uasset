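; BP_Tribble_02 is a hopping tribble creature that wanders near its spawn, eats from grain storage and damages the player on proximity.
; Tick moves it by offsets, adding a sine hop over traced ground height and separation from overlapping tribbles.
; Timers drive wandering, eating and weapon polling, switching TribbleMode to panic or burning near gunfire and flame.
; EndPlay notifies storage and game mode and spawns flesh; OnMultiply spawns two BP_Tribble_01.
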(event `self.ReceiveBeginPlay`
  (set `self.PlayerRef` (`GameplayStatics.GetPlayerCharacter` self))
  (`self.SetActorTickEnabled` true)
  (set `self.GroundZ` (.z (`self.K2_GetActorLocation`)))
  (bind (_outhit _returnvalue) (`KismetSystemLibrary.LineTraceSingle` (+ (`self.K2_GetActorLocation`) (`KismetMathLibrary.MakeVector` 0.0 0.0 50.0)) (- (`self.K2_GetActorLocation`) (`KismetMathLibrary.MakeVector` 0.0 0.0 500.0)) "TraceTypeQuery1"))
  (if _returnvalue
    (set `self.GroundZ` (+ (.z (`.Location` (`GameplayStatics.BreakHitResult` _outhit))) 46.4)))
  (bind _asbp_shooter_game_mode (cast `/Game/Variant_Shooter/Blueprints/BP_ShooterGameMode` (`GameplayStatics.GetGameMode`)))
  (`/Game/Variant_Shooter/Blueprints/BP_ShooterGameMode.TribbleSpawned` _asbp_shooter_game_mode)
  (`KismetSystemLibrary.K2_SetTimer` self "PlayHappySound" 3.0 true)
  (`KismetSystemLibrary.K2_SetTimer` self "PickNewWanderDir" 2.5 true)
  (set `self.SpawnPosition` (`self.K2_GetActorLocation`))
  (`KismetSystemLibrary.K2_SetTimer` self "CheckForPanic" 0.5 true))

(event `self.ReceiveActorBeginOverlap`
  (params (OtherActor :type "Actor Object Reference"))
  (if (== OtherActor (`self.PlayerRef`))
    (set `self.IsInProximity` true)))

(event `self.ReceiveActorEndOverlap`
  (params (OtherActor :type "Actor Object Reference"))
  (if (== OtherActor (`self.PlayerRef`))
    (set `self.IsInProximity` false)
    (set `self.DamageTimer` 0.0)))

(event `self.ReceiveTick`
  (params (DeltaSeconds :type "Float (single-precision)"))
  (bind _playerref (`self.PlayerRef`))
  (bind _grainstorageref (`self.GrainStorageRef`))
  (bind _returnvalue (- (`self.SpawnPosition`) (`self.K2_GetActorLocation`)))
  (bind _returnvalue_2 (- (`self.K2_GetActorLocation` _grainstorageref) (`self.K2_GetActorLocation`)))
  (if (`KismetSystemLibrary.IsValid` _playerref)
    (if (not (`self.IsOnFire`))
      (if (== (`self.TribbleMode`) 4)
        (`/Engine/EditorBlueprintResources/StandardMacros.IsValid` _grainstorageref
          (:`Is Valid`
            (if (> (`KismetMathLibrary.VSize` _returnvalue_2) 120.0)
              (set `self.WanderDir` (`KismetMathLibrary.MakeVector` (.x (`KismetMathLibrary.Normal` _returnvalue_2)) (.y (`KismetMathLibrary.Normal` _returnvalue_2))))
              (else
                (set `self.WanderDir` (`KismetMathLibrary.MakeVector` 0.0)))))
          (:`Is Not Valid`
            _))
        (elif (> (`KismetMathLibrary.VSize` _returnvalue) 1000.0)
          (set `self.WanderDir` (`KismetMathLibrary.Normal` _returnvalue))))
      (`self.K2_AddActorWorldOffset` (* (* (`self.WanderDir`) (150.0 150.0 150.0)) DeltaSeconds)))
    (`self.HandleSeparation` DeltaSeconds)
    (bind _output_get (set `self.HopAccumulator` (+ (`self.HopAccumulator`) DeltaSeconds)))
    (`self.K2_AddActorWorldOffset` (`KismetMathLibrary.MakeVector` 0.0 0.0 (- (+ (`self.GroundZ`) (* (`KismetMathLibrary.Abs` (`KismetMathLibrary.Sin` (* _output_get (`self.HopSpeed`)))) (`self.HopHeight`))) (.z (`self.K2_GetActorLocation`)))))
    (if (< (.z (`self.K2_GetActorLocation`)) (`self.GroundZ`))
      (`self.K2_SetActorLocation` (`KismetMathLibrary.MakeVector` (.x (`self.K2_GetActorLocation`)) (.y (`self.K2_GetActorLocation`)) (`self.GroundZ`)) false true))
    (if (`self.IsInProximity`)
      (bind _output_get_2 (set `self.DamageTimer` (+ (`self.DamageTimer`) DeltaSeconds)))
      (if (>= _output_get_2 (`self.DamageInterval`))
        (`GameplayStatics.ApplyDamage` _playerref (`self.ProximityDamage`) null self)
        (set `self.DamageTimer` 0.0)))))

(event `StartPanic`
  (bind _eatingsoundcomp (`self.EatingSoundComp`))
  (if (!= (`self.TribbleMode`) 2)
    (set `self.TribbleMode` 1)
    (`self.PickNewWanderDir`)
    (`/Engine/EditorBlueprintResources/StandardMacros.IsValid` (`self.GrainStorageRef`)
      (:`Is Valid`
        (`/Engine/EditorBlueprintResources/StandardMacros.IsValid` _eatingsoundcomp
          (:`Is Valid`
            (`AudioComponent.Stop` _eatingsoundcomp))
          (:`Is Not Valid`
            _))
        (`KismetSystemLibrary.K2_SetTimer` self "EndPanic" 5.0))
      (:`Is Not Valid`
        (`KismetSystemLibrary.K2_SetTimer` self "EndPanic" 7.0)))))

(event `EndPanic`
  (if (!= (`self.TribbleMode`) 2)
    (set `self.TribbleMode` 0)
    (`/Engine/EditorBlueprintResources/StandardMacros.IsValid` (`self.GrainStorageRef`)
      (:`Is Valid`
        (set `self.TribbleMode` 4)
        (bind _returnvalue (`GameplayStatics.SpawnSoundAttached` (`self.EatingSound`) (`self.RootComponent`) "None" (0.0 0.0 0.0) (struct) "KeepRelativeOffset" false 1.0 1.0 0.0 null null false))
        (set `self.EatingSoundComp` _returnvalue)
        (`KismetSystemLibrary.K2_SetTimer` self "DoEat" 2.0 true))
      (:`Is Not Valid`
        _))
    (`self.PickNewWanderDir`)))

(event `StartFire`
  (if (not (`self.IsOnFire`))
    (set `self.IsOnFire` true)
    (set `self.TribbleMode` 2)
    (`GameplayStatics.SpawnEmitterAttached` (`self.FireParticle`) (`self.RootComponent`))
    (bind _returnsound (`self.GetRandomFireSound`))
    (`GameplayStatics.SpawnSoundAttached` _returnsound (`self.RootComponent`) "None" (0.0 0.0 0.0) (struct) "KeepRelativeOffset" true 1.0 1.0 0.0 null null)
    (`GameplayStatics.SpawnSoundAtLocation` (`self.OnFireAmbientSound`) (`self.K2_GetActorLocation`) (struct) 1.0 1.0 0.0 null null)
    (`KismetSystemLibrary.K2_SetTimer` self "TribbleBurnDeath" 7.0)))

(event `self.ReceiveEndPlay`
  (params (EndPlayReason :type "EEndPlayReason Enum" :default "Destroyed"))
  (bind _happysoundcomp (`self.HappySoundComp`))
  (bind _grainstorageref (`self.GrainStorageRef`))
  (`KismetSystemLibrary.K2_ClearTimer` self "PlayHappySound")
  (`KismetSystemLibrary.K2_ClearTimer` self "PickNewWanderDir")
  (`KismetSystemLibrary.K2_ClearTimer` self "CheckForPanic")
  (`KismetSystemLibrary.K2_ClearTimer` self "EndPanic")
  (`KismetSystemLibrary.K2_ClearTimer` self "DoEat")
  (if (`KismetMathLibrary.InRange_IntInt` (`self.TribbleMode`) 4 4)
    (`/Engine/EditorBlueprintResources/StandardMacros.IsValid` _grainstorageref
      (:`Is Valid`
        (bind _asbp_grain_storage (cast `/Game/BluePrints/BP_GrainStorage` _grainstorageref)
          (:`then`
            (`/Game/BluePrints/BP_GrainStorage.NotifyTribbleDied` _asbp_grain_storage self))
          (:`CastFailed`
            _)))
      (:`Is Not Valid`
        _)))
  (`/Engine/EditorBlueprintResources/StandardMacros.IsValid` _happysoundcomp
    (:`Is Valid`
      (`AudioComponent.Stop` _happysoundcomp))
    (:`Is Not Valid`
      _))
  (if (not (`self.IsMultiplying`))
    (`GameplayStatics.PlaySoundAtLocation` "/Game/Soundeffects/TribbleDeath.TribbleDeath" (`self.K2_GetActorLocation`) (struct) 1.0 1.0 0.0 null null null null)
    (bind _asbp_shooter_game_mode (cast `/Game/Variant_Shooter/Blueprints/BP_ShooterGameMode` (`GameplayStatics.GetGameMode`)))
    (`/Game/Variant_Shooter/Blueprints/BP_ShooterGameMode.TribbleKilled` _asbp_shooter_game_mode)
    (bind _outactors (`GameplayStatics.GetAllActorsOfClass` "/Game/BluePrints/BP_TribbleFlesh.BP_TribbleFlesh_C"))
    (bind _returnvalue (`KismetMathLibrary.DegreesToRadians` (`KismetMathLibrary.Conv_IntToDouble` (* (`KismetArrayLibrary.Array_Length` _outactors) 60))))
    (bind _returnvalue_2 (`|SpawnActorFromClass` "/Game/BluePrints/BP_TribbleFlesh.BP_TribbleFlesh_C" (`KismetMathLibrary.MakeTransform` (+ (`self.K2_GetActorLocation`) (`KismetMathLibrary.MakeVector` (* (`KismetMathLibrary.Cos` _returnvalue) 55.0) (* (`KismetMathLibrary.Sin` _returnvalue) 55.0)))) "Undefined" "MultiplyWithRoot" null null))
    (if (`self.IsOnFire`)
      (bind _asbp_tribble_flesh (cast `/Game/BluePrints/BP_TribbleFlesh` _returnvalue_2))
      (`/Game/BluePrints/BP_TribbleFlesh.IgniteFlesh` _asbp_tribble_flesh (`self.FireParticle`)))))

(event `CustomEvent`)

(event `StartEating`
  (params (StorageRef :type "Actor Object Reference"))
  (bind _eatingsoundcomp (`self.EatingSoundComp`))
  (set `self.GrainStorageRef` StorageRef)
  (set `self.TribbleMode` 4)
  (`/Engine/EditorBlueprintResources/StandardMacros.IsValid` _eatingsoundcomp
    (:`Is Valid`
      (`AudioComponent.Stop` _eatingsoundcomp))
    (:`Is Not Valid`
      _))
  (bind _returnvalue (`GameplayStatics.SpawnSoundAttached` (`self.EatingSound`) (`self.RootComponent`) "None" (0.0 0.0 0.0) (struct) "KeepRelativeOffset" false 1.0 1.0 0.0 null null false))
  (set `self.EatingSoundComp` _returnvalue)
  (`KismetSystemLibrary.K2_SetTimer` self "DoEat" 2.0 true))

(event `StopEating`
  (bind _eatingsoundcomp (`self.EatingSoundComp`))
  (set `self.TribbleMode` 0)
  (set `self.GrainStorageRef` null)
  (`/Engine/EditorBlueprintResources/StandardMacros.IsValid` _eatingsoundcomp
    (:`Is Valid`
      (`AudioComponent.Stop` _eatingsoundcomp)
      (set `self.EatingSoundComp` null))
    (:`Is Not Valid`
      _))
  (`KismetSystemLibrary.K2_ClearTimer` self "DoEat"))

(fn `CheckForPanic`
  (bind _returnvalue (`KismetMathLibrary.VSize` (- (`self.K2_GetActorLocation`) (`self.K2_GetActorLocation` (`GameplayStatics.GetPlayerCharacter` 0)))))
  (if (> _returnvalue 2000.0)
    (return)
    (else
      (`|ExecutionSequence`
        (:`then_0`
          (bind _outactors (`GameplayStatics.GetAllActorsOfClass` "/Game/BluePrints/BP_ShooterWeapon_Flamethrower.BP_ShooterWeapon_Flamethrower_C"))
          (bind _output (`|GetArrayItem` _outactors))
          (`/Engine/EditorBlueprintResources/StandardMacros.IsValid` _output
            (:`Is Valid`
              (bind _asbp_shooter_weapon_flamethrower (cast `/Game/BluePrints/BP_ShooterWeapon_Flamethrower` _output))
              (if (`/Game/BluePrints/BP_ShooterWeapon_Flamethrower.IsCurrentlyFiring` _asbp_shooter_weapon_flamethrower)
                (`self.StartPanic`)
                (if (< _returnvalue 600.0)
                  (`self.StartFire`))))))
        (:`then_1`
          (bind _outactors_2 (`GameplayStatics.GetAllActorsOfClass` "/Game/BluePrints/BP_ShooterWeapon_Shotgun.BP_ShooterWeapon_Shotgun_C"))
          (bind _output_2 (`|GetArrayItem` _outactors_2))
          (`/Engine/EditorBlueprintResources/StandardMacros.IsValid` _output_2
            (:`Is Valid`
              (bind _asbp_shooter_weapon_base (cast `/Game/Variant_Shooter/Blueprints/Pickups/BP_ShooterWeaponBase` _output_2))
              (if (< (- (`GameplayStatics.GetTimeSeconds`) (`/Game/Variant_Shooter/Blueprints/Pickups/BP_ShooterWeaponBase.Time of Last Shot` _asbp_shooter_weapon_base)) 0.5)
                (`self.StartPanic`)))))))))

(fn `DoEat`
  (bind _grainstorageref (`self.GrainStorageRef`))
  (if (== (`self.TribbleMode`) 4)
    (`/Engine/EditorBlueprintResources/StandardMacros.IsValid` _grainstorageref
      (:`Is Valid`
        (bind _asbp_grain_storage (cast `/Game/BluePrints/BP_GrainStorage` _grainstorageref))
        (`/Game/BluePrints/BP_GrainStorage.EatGrain` _asbp_grain_storage)))))

(fn `GetRandomFireSound`
  (returns (ReturnSound :type "SoundBase Object Reference"))
  (locals (Sounds :type "Array of SoundBase Object Reference"))
  (bind _sounds (`local.Sounds`))
  (`KismetArrayLibrary.Array_Add` _sounds (`self.FireSound1`))
  (`KismetArrayLibrary.Array_Add` _sounds (`self.FireSound2`))
  (`KismetArrayLibrary.Array_Add` _sounds (`self.FireSound3`))
  (`KismetArrayLibrary.Array_Add` _sounds (`self.FireSound4`))
  (return (`KismetArrayLibrary.Array_Random` _sounds)))

(fn `HandleSeparation`
  (params (DeltaSeconds :type "Float (single-precision)"))
  (bind _tribble_colider (`self.Tribble_Colider`))
  (`/Engine/EditorBlueprintResources/StandardMacros.IsValid` _tribble_colider
    (:`Is Valid`
      (set `self.CachedOverlapping` (`PrimitiveComponent.GetOverlappingActors` _tribble_colider (`GameplayStatics.GetObjectClass` self)))
      (for _array_element (`self.CachedOverlapping`)
        (`/Engine/EditorBlueprintResources/StandardMacros.IsValid` _array_element
          (:`Is Valid`
            (`self.K2_AddActorWorldOffset` (* (`KismetMathLibrary.MakeVector` (.x (`KismetMathLibrary.Normal` (+ (- (`self.K2_GetActorLocation`) (`self.K2_GetActorLocation` _array_element)) (`KismetMathLibrary.MakeVector` (`KismetMathLibrary.RandomFloatInRange` -10.0 10.0) (`KismetMathLibrary.RandomFloatInRange` -10.0 10.0))))) (.y (`KismetMathLibrary.Normal` (+ (- (`self.K2_GetActorLocation`) (`self.K2_GetActorLocation` _array_element)) (`KismetMathLibrary.MakeVector` (`KismetMathLibrary.RandomFloatInRange` -10.0 10.0) (`KismetMathLibrary.RandomFloatInRange` -10.0 10.0)))))) (* (`self.SeparationForce`) DeltaSeconds)))))))))

(fn `OnMultiply`
  (bind _returnvalue (`self.K2_GetActorLocation`))
  (`|SpawnActorFromClass` "/Game/BluePrints/BP_Tribble_01.BP_Tribble_01_C" (`KismetMathLibrary.MakeTransform` (+ _returnvalue (`KismetMathLibrary.MakeVector` (`KismetMathLibrary.RandomFloatInRange` -150.0 150.0) (`KismetMathLibrary.RandomFloatInRange` -150.0 150.0)))) "Undefined" "MultiplyWithRoot" null null)
  (`|SpawnActorFromClass` "/Game/BluePrints/BP_Tribble_01.BP_Tribble_01_C" (`KismetMathLibrary.MakeTransform` (+ _returnvalue (`KismetMathLibrary.MakeVector` (`KismetMathLibrary.RandomFloatInRange` -150.0 150.0) (`KismetMathLibrary.RandomFloatInRange` -150.0 150.0)))) "Undefined" "MultiplyWithRoot" null null))

(fn `PickNewWanderDir`
  (set `self.WanderDir` (`KismetMathLibrary.Normal` (`KismetMathLibrary.MakeVector` (`KismetMathLibrary.RandomFloatInRange` -1.0 1.0) (`KismetMathLibrary.RandomFloatInRange` -1.0 1.0)))))

(fn `PlayHappySound`
  (if (`KismetMathLibrary.InRange_IntInt` (`self.TribbleMode`) 0 0)
    (bind _returnvalue (`GameplayStatics.SpawnSoundAttached` (`self.HappySound`) (`self.RootComponent`) "None" (0.0 0.0 0.0) (struct) "KeepRelativeOffset" true 1.0 1.0 0.0 null null))
    (set `self.HappySoundComp` _returnvalue)))

(fn `TribbleBurnDeath`
  (bind _asactor (castclass `Actor` (`self.TribbleAshesClass`)))
  (bind _returnvalue (`|SpawnActorFromClass` _asactor (`KismetMathLibrary.MakeTransform` (`self.K2_GetActorLocation`)) "Undefined" "MultiplyWithRoot" null null))
  (bind _asbp_tribble_flesh (cast `/Game/BluePrints/BP_TribbleFlesh` _returnvalue)
    (:`then`
      (`/Game/BluePrints/BP_TribbleFlesh.IgniteFlesh` _asbp_tribble_flesh (`self.FireParticle`)))
    (:`CastFailed`
      _))
  (`self.K2_DestroyActor`))

(fn `UserConstructionScript`
  (set `self.WanderDir` (`KismetMathLibrary.MakeVector` 1.0)))