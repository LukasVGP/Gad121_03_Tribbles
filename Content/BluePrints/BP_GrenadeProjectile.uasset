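; Grenade projectile that explodes on its first actor overlap and sets nearby Tribbles on fire.
; A one-shot flag guards the overlap event, which spawns an explosion effect and sound, then runs a sphere overlap for WorldDynamic objects around the impact.
; Actors tagged Tribble are cast to either of two Tribble Blueprint variants to call StartFire, and the grenade then destroys itself.
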(event `self.ReceiveActorBeginOverlap`
  (params (OtherActor :type "Actor Object Reference"))
  (bind _returnvalue (`self.K2_GetActorLocation`))
  (if (not (`self.HasProcessedHit`))
    (set `self.HasProcessedHit` true)
    (`GameplayStatics.SpawnEmitterAtLocation` "/Game/StarterContent/Particles/P_Explosion.P_Explosion" _returnvalue (struct) (3.0 3.0 3.0))
    (`GameplayStatics.SpawnSoundAtLocation` "/Game/StarterContent/Audio/Explosion_Cue.Explosion_Cue" _returnvalue (struct) 1.0 1.0 0.0 null null)
    (bind _outactors (`KismetSystemLibrary.SphereOverlapActors` self _returnvalue 600.0 (`|MakeArray` (enumliteral `EObjectTypeQuery` "ObjectTypeQuery2"))))
    (for _array_element _outactors
      (if (`self.ActorHasTag` _array_element "Tribble")
        (bind _asbp_tribble_03 (cast `/Game/BluePrints/BP_Tribble_03` _array_element)
          (:`then`
            (`/Game/BluePrints/BP_Tribble_03.StartFire` _asbp_tribble_03))
          (:`CastFailed`
            (bind _asbp_tribble_04 (cast `/Game/BluePrints/BP_Tribble_04` _array_element))
            (`/Game/BluePrints/BP_Tribble_04.StartFire` _asbp_tribble_04)))))
    (`/Engine/EditorBlueprintResources/StandardMacros.IsValid` self
      (:`Is Valid`
        (`self.K2_DestroyActor` self)))))

(fn `UserConstructionScript`)